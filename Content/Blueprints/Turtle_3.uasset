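; Turtle_3 is a turtle actor that calls Movement every tick while its Speed periodically flips sign.
; Two looping timers of equal period set Speed to the stored default and to its negative.
; A delay after BeginPlay applies the first reversal and offsets the second timer, so the positive phase lasts longer than the negative one in the repeating cycle.
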(event Custom|SpeedChange1
  (Variables|Default|SetSpeed (* -1 (Variables|Default|GetDefaultSpeed))))

(event Custom|SpeedChange
  (Variables|Default|SetSpeed (Variables|Default|GetDefaultSpeed)))

(event EventBeginPlay
  (Variables|Default|SetbIsFirstStep true)
  (Variables|Default|SetDefaultSpeed (Variables|Default|GetSpeed))
  (Utilities|Time|SetTimerbyEvent (delegate Custom|SpeedChange) 1.5 true)
  (if (Variables|Default|GetbIsFirstStep)
    (Variables|Default|SetbIsFirstStep false)
    (Utilities|FlowControl|Delay 1.0)
    (Variables|Default|SetSpeed (* -1 (Variables|Default|GetDefaultSpeed))))
  (Utilities|Time|SetTimerbyEvent (delegate Custom|SpeedChange1) 1.5 true))

(event Collision|EventActorBeginOverlap
  (params (OtherActor :type Actor%20Object%20Reference)))

(event EventTick
  (params (DeltaSeconds :type Float%20%28single-precision%29))
  (Class|Turtle|Movement))

(fn ConstructionScript)